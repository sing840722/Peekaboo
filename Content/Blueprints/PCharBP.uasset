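; PCharBP is a Blueprint, apparently a player character, with events for damaging hit targets and marking team deaths.
; Destructable applies point damage to a supplied hit's actor, while DeathEffects calls SpawnEffects to place a red or blue decal at the target's location by Team.
; BeginPlay saves the Cube's scale and shrinks it to zero.
; A timeline that would expand the Cube is never triggered.
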(event `self.ReceiveBeginPlay`
  (bind _cube (`self.Cube`))
  (set `self.VectorTarget` (`SceneComponent.RelativeScale3D` _cube))
  (`SceneComponent.SetWorldScale3D` _cube (0.0 0.0 0.0)))

(event `Key|E`
  (params (Key :type "Key Structure" :default "AnyKey")))

(event `self.Destructable`
  (params (Target :type "HitResult Structure"))
  (bind (_bblockinghit _binitialoverlap _time _location _impactpoint _normal _impactnormal _physmat _hitactor _hitcomponent _hitbonename _hititem _tracestart) (`GameplayStatics.BreakHitResult` Target))
  (`GameplayStatics.ApplyPointDamage` _hitactor 10.0 _tracestart Target null self "/Script/Engine.DamageType"))

(event `self.DeathEffects`
  (params (Target :type "PChar Object Reference"))
  (`self.spawn effects` Target))

(event `spawn effects`
  (params (NewParam :type "PChar Object Reference"))
  (bind _returnvalue (`self.K2_GetActorLocation` NewParam))
  (if (== (`PChar.Team` NewParam) (`KismetTextLibrary.Conv_StringToText` "Red"))
    (`GameplayStatics.SpawnDecalAtLocation` "/Game/FinishedArt/Death/Decal/Death_Decal_RED_MAT.Death_Decal_RED_MAT" (500.0 500.0 500.0) _returnvalue (struct :`Pitch` -90.0) 0.0)
    (else
      (`GameplayStatics.SpawnDecalAtLocation` "/Game/FinishedArt/Death/Decal/Death_Decal_BLUE_MAT.Death_Decal_BLUE_MAT" (500.0 500.0 500.0) _returnvalue (struct :`Pitch` -90.0) 0.0))))

(fn `UserConstructionScript`)