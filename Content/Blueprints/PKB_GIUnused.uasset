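; Game instance Blueprint, named as unused, that handles the main menu and LAN session flow: host, search, join, leave and quit.
; Hosting opens LightingTestC as a listen server, and searching fills a server list widget with one entry per result.
; Joining checks for a free slot first, and leaving destroys the session and returns to the GUI level.
; Failures only print messages; the HUD event is empty and the Lobby widget code is unconnected.
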(event `Instance ShowMainMenu`
  (bind _returnvalue (`|CreateWidget` "/Game/InProgress/Moses/GraphicalUserInterface/MainMenu/MainMenu_BP.MainMenu_BP_C" (`GameplayStatics.GetPlayerController` 0)))
  (`UserWidget.AddToViewport` _returnvalue 0))

(event `Instance HostGame`
  (`CreateSessionCallbackProxy.CreateSession` (`GameplayStatics.GetPlayerController` 0) 5 true
    (:`OnSuccess`
      (`GameplayStatics.OpenLevel` (`self.Lighting_Test_c`) true "listen"))
    (:`OnFailure`
      (`KismetSystemLibrary.PrintString` "Failed to create session"))))

(event `Instance SearchGame`
  (bind _results (`FindSessionsCallbackProxy.FindSessions` (`GameplayStatics.GetPlayerController` 0) 5 true)
    (:`OnSuccess`
      (bind _returnvalue (`|CreateWidget` "/Game/InProgress/Moses/GraphicalUserInterface/MainMenu/ServerList_BP.ServerList_BP_C"))
      (`UserWidget.AddToViewport` _returnvalue 0)
      (for _array_element _results
        (bind _returnvalue_2 (`|CreateWidget` "/Game/InProgress/Moses/GraphicalUserInterface/MainMenu/ServerInformation_BP.ServerInformation_BP_C"))
        (set `/Game/InProgress/Moses/GraphicalUserInterface/MainMenu/ServerInformation_BP.Server` _array_element _returnvalue_2)
        (`VerticalBox.AddChildToVerticalBox` (`/Game/InProgress/Moses/GraphicalUserInterface/MainMenu/ServerList_BP.ResultList` _returnvalue) _returnvalue_2)))
    (:`OnFailure`
      (`KismetSystemLibrary.PrintString` "Failed to find Session"))))

(event `Instance JoinGame`
  (params (`Target Server` :type "BlueprintSessionResult Structure"))
  (if (< (`FindSessionsCallbackProxy.GetCurrentPlayers` `Target Server`) (`FindSessionsCallbackProxy.GetMaxPlayers` `Target Server`))
    (`JoinSessionCallbackProxy.JoinSession` (`GameplayStatics.GetPlayerController` 0) `Target Server`
      (:`OnSuccess`
        (`KismetSystemLibrary.PrintString` "Joined Server"))
      (:`OnFailure`
        (`KismetSystemLibrary.PrintString` "Failed to Join Server")))
    (else
      (`KismetSystemLibrary.PrintString` "Server is full"))))

(event `Instance LeaveGame`
  (`DestroySessionCallbackProxy.DestroySession` (`GameplayStatics.GetPlayerController` 0)
    (:`OnSuccess`
      (`GameplayStatics.OpenLevel` "GUI"))
    (:`OnFailure`
      (`KismetSystemLibrary.PrintString` "Failed To Leave Game"))))

(event `Instance QuitGame`
  (`KismetSystemLibrary.ExecuteConsoleCommand` "QUIT"))

(event `Instance ShowWhatTheTimeHUD`)